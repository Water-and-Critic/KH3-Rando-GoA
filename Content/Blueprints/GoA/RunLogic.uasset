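; RunLogic is a bootstrap actor that spawns the GoA gameplay logic actors at runtime.
; On BeginPlay, if no save point logic actor exists, it spawns one plus event, level-up, bonus level and retry logic actors at the player controller's transform.
; Every Tick, it pushes placeholder test text, built with the level package names as parameters, to the Tres information window and pause hint.
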(event EventBeginPlay
  (bind _returnvalue (Game|GetPlayerController 0))
  (bind _returnvalue_2 (Transformation|GetActorTransform _returnvalue))
  (bind _outactors (Actor|GetAllActorsOfClass "/Game/Blueprints/GoA/Actors/A_GoA_SavePoint_Logic.A_GoA_SavePoint_Logic_C"))
  (if (not (> (Utilities|Array|Length _outactors) 0))
    (Game|SpawnActorfromClass "/Game/Blueprints/GoA/Actors/A_GoA_SavePoint_Logic.A_GoA_SavePoint_Logic_C" _returnvalue_2 "Undefined" 0 0)
    (Game|SpawnActorfromClass "/Game/Mods/KH3Randomizer/EventActor.EventActor_C" _returnvalue_2 "Undefined" 0 0)
    (Game|SpawnActorfromClass "/Game/Mods/KH3Randomizer/LevelUpActor.LevelUpActor_C" _returnvalue_2 "Undefined" 0 0)
    (Game|SpawnActorfromClass "/Game/Mods/KH3Randomizer/VBonusLevelActor.VBonusLevelActor_C" _returnvalue_2 "Undefined" 0 0)
    (Game|SpawnActorfromClass "/Game/Mods/KH3Randomizer/RetryLogicActor.RetryLogicActor_C" _returnvalue_2 "Undefined" 0 0)))

(event EventTick
  (params (DeltaSeconds :type Float%20%28single-precision%29))
  (bind _returnvalue (Class|TresUnrealEngineLevelStatics|GetLevelPackageNames false))
  (bind _tresloctext (Utilities|Struct|MakeTresLocText "" "" _returnvalue "TESTTESTTESTTEST"))
  (Class|TresGameBlueprintLibrary|TresUIOpenInformation _tresloctext false 1.0)
  (Class|TresGameBlueprintLibrary|TresUISetPauseHintText _tresloctext))

(fn ConstructionScript)